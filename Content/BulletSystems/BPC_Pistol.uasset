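; Bullet component that drives its owning actor as a simulated pistol projectile with gravity drop.
; BeginPlay sets velocity from the owner's forward vector and starts both a lifespan countdown and a delay-driven movement loop.
; Each step line-traces the next segment, destroying the owner on a hit or else moving it to the segment end and applying mass-based gravity to velocity.
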(event `self.ReceiveBeginPlay`
  (bind _returnvalue (`self.GetOwner`))
  (bind _returnvalue_2 (`self.GetOwner`))
  (bind _returnvalue_3 (`Actor.K2_GetActorLocation` _returnvalue))
  (bind (_startpos _endpos) (`/Game/BulletSystems/BP_BulletBallisticsFunctions.Find Start & End Position` _returnvalue_3 (`self.Velocity`) (`self.DeltaTime`)))
  ;[1 1 1] Shooting (Default Left Mouse Button)
  (`|ExecutionSequence`
    (:`then_0`
      ;;[1 1 1] Prepare Variables for use at start
      (set `self.Velocity` (* (`Actor.GetActorForwardVector` _returnvalue) (`self.BulletSpeed`)))
      (set `self.StartPos` _returnvalue_3)
      (`KismetArrayLibrary.Array_Add` (`self.IgnoreActor`) _returnvalue)
      (`KismetSystemLibrary.Delay` (`self.LifeSpan`))
      (`Actor.K2_DestroyActor` _returnvalue))
    (:`then_1`
      ;;[1 1 1] Shooting Liune Trace affected by Gravity
      (set `self.StartPos` _startpos :!label _label)
      (set `self.EndPos` _endpos)
      (bind (_returnvalue_4 _outhit) (`/Game/BulletSystems/BP_BulletBallisticsFunctions.Spawn Line Trace` _startpos _endpos (`self.IgnoreActor`)))
      (if _returnvalue_4
        (`Actor.K2_DestroyActor` _returnvalue_2)
        (bind _output_get (set `self.Out Hit` _outhit))
        (else
          (`Actor.K2_SetActorLocation` _returnvalue_2 (`self.EndPos`) false false)
          (set `self.Velocity` (`/Game/BulletSystems/BP_BulletBallisticsFunctions.Apply Gravity` (`self.Velocity`) (`self.BulletMass`) (`self.DeltaTime`)))
          (`KismetSystemLibrary.Delay` (`self.UpdateBullet`))
          (`KismetSystemLibrary.PrintString` (`KismetStringLibrary.Conv_DoubleToString` (`.Distance` (`GameplayStatics.BreakHitResult` _output_get))))
          (goto _label))))))