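; Bullet ballistics helper functions that simulate a projectile with line traces and gravity drop.
; FindStartEndPosition projects a segment's end from start, velocity and delta time.
; SpawnLineTrace traces a given segment on the Visibility channel with an ignore list and persistent debug drawing, returning the hit.
; ApplyGravity lowers vertical velocity over delta time, scaling gravitational acceleration by bullet mass, so heavier bullets drop faster.
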(fn `Apply Gravity`
  (params (`Velocity In` :type "Vector Structure") (`Bullet Mass` :type "Float (double-precision)") (DeltaTime :type "Float (double-precision)"))
  (returns (VelocityOut :type "Vector Structure"))
  ;[1 1 1] Decreases Velocity vectors z value by gravity * Bullet Mass * Delta Time - Velocity
  (return (- `Velocity In` (* (`KismetMathLibrary.MakeVector` 0.0 0.0 (* 980.0 `Bullet Mass`)) DeltaTime))))

(fn `Find Start & End Position`
  (params (Start :type "Vector Structure") (Velocity :type "Vector Structure") (DeltaTime :type "Float (double-precision)"))
  (returns (StartPos :type "Vector Structure") (EndPos :type "Vector Structure"))
  ;[1 1 1] Finds the start and end position of the line trace
  (return Start (+ Start (* Velocity DeltaTime))))

(fn `Spawn Line Trace`
  (params (Start :type "Vector Structure") (End :type "Vector Structure") (ActorsToIgnore :type "Array of Actor Object Reference (by ref)"))
  (returns (ReturnValue :type Boolean) (OutHit :type "HitResult Structure"))
  ;[1 1 1] Shoots the line trace
  (bind (_outhit _returnvalue) (`KismetSystemLibrary.LineTraceSingle` null Start End "TraceTypeQuery1" false ActorsToIgnore "Persistent"))
  (return _returnvalue _outhit))