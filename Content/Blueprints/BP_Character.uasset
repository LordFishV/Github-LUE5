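; BP_Character is a player character Blueprint with basic movement, look controls and shooting.
; Axis inputs add movement along the actor's forward and right vectors and feed look input into controller pitch and yaw.
; Pressing Shoot spawns a BP_Bullet at the world transform of the Sphere component, which acts as the muzzle point.
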(event `InputAxis|Move Forward/Back`
  (params (AxisValue :type "Float (single-precision)"))
  (`self.AddMovementInput` (`self.GetActorForwardVector`) AxisValue))

(event `InputAxis|Look Up/Down`
  (params (AxisValue :type "Float (single-precision)"))
  (`self.AddControllerPitchInput` AxisValue))

(event `InputAxis|Look Right/Left`
  (params (AxisValue :type "Float (single-precision)"))
  (`self.AddControllerYawInput` AxisValue))

(event `InputAxis|Move Right/Left`
  (params (AxisValue :type "Float (single-precision)"))
  (`self.AddMovementInput` (`self.GetActorRightVector`) AxisValue))

(event `InputAction|Shoot`
  (params (Key :type "Key Structure"))
  (:`Pressed`
    (`|SpawnActorFromClass` "/Game/Blueprints/BP_Bullet.BP_Bullet_C" (`SceneComponent.K2_GetComponentToWorld` (`self.Sphere`)) "Undefined" "MultiplyWithRoot" null null)))

(fn `UserConstructionScript`)